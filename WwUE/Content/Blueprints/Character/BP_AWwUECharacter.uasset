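; Player character Blueprint with debug keys for exercising weapon firing and fire rate.
; Key 1 fires for a set number of ticks using a next-tick delay loop, while the bracket keys start and stop firing manually.
; Keys 2 and 3 lower and raise the fire interval in small steps.
; The construction script, rather than BeginPlay, creates the weapon HUD widget, adds it to the viewport and initializes it with this character.
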(event EventBeginPlay)

(event Input|KeyboardEvents|RightBracket
  (params (Key :type Key%20Structure :default "None"))
  (:Pressed
    (Class|WwUECharacter|StopFiring (Class|EnhancedInputLibrary|MakeInputActionValueOfType 0.0 0.0 0.0 "Boolean"))))

(event Input|KeyboardEvents|LeftBracket
  (params (Key :type Key%20Structure :default "None"))
  (:Pressed
    (Class|WwUECharacter|StartFiring (Class|EnhancedInputLibrary|MakeInputActionValueOfType 0.0 0.0 0.0 "Boolean"))))

(event Input|KeyboardEvents|1
  (params (Key :type Key%20Structure :default "None"))
  (bind _returnvalue (Class|EnhancedInputLibrary|MakeInputActionValueOfType 0.0 0.0 0.0 "Boolean"))
  (:Pressed
    (Class|WwUECharacter|StartFiring _returnvalue)
    (if (< (Variables|Default|GetTicks%20Waited) (Variables|Default|GetTicks%20To%20Wait)) :!label _label
      (Utilities|FlowControl|DelayUntilNextTick)
      (Math|Integer|IncrementInt (Variables|Default|GetTicks%20Waited)
        (:%20%20
          (goto _label)))
      (else
        (Class|WwUECharacter|StopFiring _returnvalue)
        (Variables|Default|SetTicks%20Waited 0)))))

(event Input|KeyboardEvents|3
  (params (Key :type Key%20Structure :default "None"))
  (:Pressed
    (Class|WwUECharacter|SetFireInterval (+ (Class|WwUECharacter|GetFireInterval) 0.01))))

(event Input|KeyboardEvents|2
  (params (Key :type Key%20Structure :default "None"))
  (:Pressed
    (Class|WwUECharacter|SetFireInterval (- (Class|WwUECharacter|GetFireInterval) 0.01))))

(fn ConstructionScript
  (bind _returnvalue (Game|ConstructObjectfromClass "/Game/Blueprints/WBP_WeaponHUD.WBP_WeaponHUD_C"))
  (UserInterface|Viewport|AddtoViewport _returnvalue 0)
  (Default|Init _returnvalue self))