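; Ambience zone actor that triggers play and stop as the player comes within or leaves audible range.
; Tick measures the first player camera manager's distance to the actor origin against a fixed radius, calling OnTriggerPlay or OnTriggerStop only on changes.
; Box overlaps separately forward actors to OnActorEnter and OnActorExit.
; BeginPlay sets the occlusion refresh interval, and construction applies the box's in-game visibility setting.
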(event OnComponentBeginOverlap(Box)
  (params (OverlappedComponent :type Primitive%20Component%20Object%20Reference) (OtherActor :type Actor%20Object%20Reference) (OtherComp :type Primitive%20Component%20Object%20Reference) (OtherBodyIndex :type Integer) (bFromSweep :type Boolean) (SweepResult :type Hit%20Result%20Structure%20%28by%20ref%29))
  (Class|WwUEAmbienceZone|OnActorEnter OtherActor))

(event OnComponentEndOverlap(Box)
  (params (OverlappedComponent :type Primitive%20Component%20Object%20Reference) (OtherActor :type Actor%20Object%20Reference) (OtherComp :type Primitive%20Component%20Object%20Reference) (OtherBodyIndex :type Integer))
  (Class|WwUEAmbienceZone|OnActorExit OtherActor))

(event EventBeginPlay
  (Class|AkGameplayStatics|SetOcclusionRefreshInterval 0.0 self))

(event Collision|EventActorBeginOverlap
  (params (OtherActor :type Actor%20Object%20Reference)))

(event EventTick
  (params (DeltaSeconds :type Float%20%28single-precision%29))
  (bind _returnvalue (Game|GetPlayerCameraManager 0))
  (bind _in_audible_distance (CallFunction|IsActorinAudibleDistance _returnvalue))
  ;[1 1 1] Don't continue if player cam is null
  (Utilities|IsValid (Game|GetPlayerCameraManager 0)
    (:Is%20Valid
      (Utilities|FlowControl|Sequence
        (:then_0
          (if (!= (Variables|Default|GetIs%20Player%20In%20Audible%20Distance) _in_audible_distance)
            (if _in_audible_distance
              (Class|WwUEAmbienceZone|OnTriggerPlay _returnvalue)
              (else
                (Class|WwUEAmbienceZone|OnTriggerStop _returnvalue))))
          (Variables|Default|SetIs%20Player%20In%20Audible%20Distance _in_audible_distance))))))

(fn ConstructionScript
  (Utilities|FlowControl|Sequence
    (:then_0
      (Development|SetHiddeninGame (Variables|Default|GetBox) (Variables|Sound|GetHidden%20In%20Game) false))))

(fn IsActorinAudibleDistance
  (params (Actor :type Actor%20Object%20Reference%20%28by%20ref%29))
  (return (<= (Transformation|GetDistanceTo Actor self) 1e+03)))