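; Ambience zone Blueprint outlined by a spline, meant to track whether the player's camera is inside it; it appears unfinished.
; BeginPlay caches the player camera manager, and Tick compares IsActorInside against IsPlayerInside, storing the inequality result rather than the inside state.
; IsActorInside only stores the actor's location, with its return node unconnected.
; The construction script adds one spline mesh component and loops over spline points with an empty body.
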(event EventBeginPlay
  (bind _returnvalue (Game|GetPlayerCameraManager 0))
  (Utilities|FlowControl|Sequence
    (:then_0
      (Utilities|IsValid _returnvalue
        (:Is%20Valid
          (Variables|Default|SetTarget%20Actor _returnvalue))))))

(event EventTick
  (params (DeltaSeconds :type Float%20%28single-precision%29))
  ;[1 1 1] Halt execution if our target actor isn't valid
  (Utilities|IsValid (Variables|Default|GetTarget%20Actor)
    (:Is%20Valid
      (Utilities|FlowControl|Sequence
        (:then_0
          (if (!= (.Is%20Inside (AmbienceZoneSpline|Util|IsActorInside (Variables|Default|GetTarget%20Actor))) (Variables|AmbienceZoneSpline|GetIs%20Player%20Inside))
            (Variables|AmbienceZoneSpline|SetIs%20Player%20Inside (!= (.Is%20Inside (AmbienceZoneSpline|Util|IsActorInside (Variables|Default|GetTarget%20Actor))) (Variables|AmbienceZoneSpline|GetIs%20Player%20Inside)))))))))

(fn ConstructionScript
  (bind _returnvalue (AddComponent|AddSplineMeshComponent false))
  (Variables|Default|SetSpline%20Mesh _returnvalue)
  (for _index (range 0 (Spline|GetNumberOfSplinePoints (Variables|Default|GetSpline)))
    _))

(fn IsActorInside
  (params (Actor :type Actor%20Object%20Reference%20%28by%20ref%29))
  (Utilities|FlowControl|Sequence
    (:then_0
      ;[1 1 1] Store Actor Location
      (LocalVariables|SetActor%20Location (Transformation|GetActorLocation Actor)))))