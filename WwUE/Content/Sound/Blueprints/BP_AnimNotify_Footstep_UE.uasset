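; Footstep anim notify that plays a sound chosen by the physical surface under a named socket on the animated mesh.
; On notify, it traces down from the socket on the Visibility channel, ignoring the mesh's owner, and switches on the hit's surface type.
; Grass, mud, concrete, wood and a default each select a sound, apparently placeholder editor sounds, which is passed to SpawnSoundAttached with the socket's name and location.
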(fn ReceivedNotify
  (params (MeshComp :type Skeletal%20Mesh%20Component%20Object%20Reference) (Animation :type Anim%20Sequence%20Base%20Object%20Reference) (EventReference :type Anim%20Notify%20Event%20Reference%20Structure%20%28by%20ref%29))
  (bind _attach_name (Variables|Default|GetAttach%20Name))
  (bind _returnvalue (Transformation|GetSocketLocation MeshComp _attach_name))
  (bind _output_get (LocalVariables|SetSocket%20Location _returnvalue))
  (bind _outhit (Collision|LineTraceByChannel _output_get (- _returnvalue (Math|Vector|MakeVector 0.0 0.0 (Variables|Default|GetLine%20Trace%20Distance))) "TraceTypeQuery1" false (Utilities|Array|MakeArray (Components|GetOwner MeshComp)) "None"))
  (switch Utilities|FlowControl|Switch|SwitchonEPhysicalSurface (Variables|/Script/PhysicsCore.PhysicalMaterial|GetSurfaceType (.PhysMat (Collision|BreakHitResult _outhit)))
    (:SurfaceType_Default
      (LocalVariables|SetSound "/Engine/VREditor/Sounds/UI/Gizmo_Handle_Clicked.Gizmo_Handle_Clicked"))
    (:SurfaceType1
      (LocalVariables|SetSound "/Engine/VREditor/Sounds/UI/Object_PickUp.Object_PickUp"))
    (:SurfaceType2
      (LocalVariables|SetSound "/Engine/VREditor/Sounds/VR_confirm.VR_confirm"))
    (:SurfaceType3
      (LocalVariables|SetSound "/Engine/EditorSounds/Notifications/CompileFailed.CompileFailed"))
    (:SurfaceType4
      (LocalVariables|SetSound "/Engine/EditorSounds/Notifications/CompileSuccess.CompileSuccess")))
  (Audio|SpawnSoundAttached (LocalVariables|GetSound) 0 (Variables|Default|GetAttach%20Name) (LocalVariables|GetSocket%20Location) "0, 0, 0" "KeepRelativeOffset" false 1.0 1.0 0.0 0 0))