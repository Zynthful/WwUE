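; Anim notify that posts a Wwise AkEvent from an animation.
; With PostAttached set, it posts on an Ak component attached to the mesh at AttachPointName; otherwise it fires the event at the mesh's world location with zero orientation.
; The notify name displays as an SND tag with the event's name in brackets.
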(fn ReceivedNotify
  (params (MeshComp :type Skeletal%20Mesh%20Component%20Object%20Reference) (Animation :type Anim%20Sequence%20Base%20Object%20Reference) (EventReference :type Anim%20Notify%20Event%20Reference%20Structure%20%28by%20ref%29))
  (if (Variables|Sound|GetPost%20Attached)
    (bind _returnvalue (Class|AkGameplayStatics|GetAkComponent MeshComp (Variables|Sound|GetAttach%20Point%20Name) "0, 0, 0" "KeepRelativeOffset"))
    (Class|AkGameObject|PostAkEvent _returnvalue (Variables|Sound|GetAk%20Event))
    (else
      (Class|AkGameplayStatics|PostEventatLocation (Variables|Sound|GetAk%20Event) (Transformation|GetWorldLocation MeshComp) "0, 0, 0"))))

(fn GetNotifyName
  (return (Utilities|String|Append "SND" " [" (Utilities|GetDisplayName (Variables|Sound|GetAk%20Event)) "]")))