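; Wwise footstep anim notify that plays a surface-dependent sound from an Ak component at the configured attach point on the animated mesh.
; A downward visibility trace from that component reads the physical material's surface type and sets it as a Wwise switch before posting.
; The footstep type selects the event and notify name; only Step has an event, a test beep, while Jump, Land and Pivot are empty.
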(fn ReceivedNotify
  (params (MeshComp :type Skeletal%20Mesh%20Component%20Object%20Reference) (Animation :type Anim%20Sequence%20Base%20Object%20Reference) (EventReference :type Anim%20Notify%20Event%20Reference%20Structure%20%28by%20ref%29))
  (Utilities|FlowControl|Sequence
    (:then_0
      ;[1 1 1] Get Ak Component
      (bind _returnvalue (Class|AkGameplayStatics|GetAkComponent MeshComp (Variables|Default|GetAttach%20Name) "0, 0, 0" "KeepRelativeOffset"))
      (Utilities|IsValid _returnvalue
        (:Is%20Valid
          (LocalVariables|SetAkComponent _returnvalue))
        (:Is%20Not%20Valid
          (return false))))
    (:then_1
      ;[1 1 1] Set SurfaceType AkSwitch
      (if (.Has%20Hit (CallFunction|GetSurfaceType (LocalVariables|GetAkComponent)))
        (Class|AkComponent|SetSwitch (LocalVariables|GetAkComponent) 0 (Variables|Default|GetSurface%20Type%20Switch%20Group%20Name) (Utilities|String|EnumtoString (.Surface%20Type (CallFunction|GetSurfaceType (LocalVariables|GetAkComponent)))))))
    (:then_2
      ;[1 1 1] Post Event
      (CallFunction|PostEvent (LocalVariables|GetAkComponent)))))

(fn GetSurfaceType
  (params (Ak%20Component :type Ak%20Component%20Object%20Reference%20%28by%20ref%29))
  (bind _returnvalue (Transformation|GetWorldLocation Ak%20Component))
  (bind (_outhit _returnvalue_2) (Collision|LineTraceByChannel _returnvalue (- _returnvalue (Math|Vector|MakeVector 0.0 0.0 (Variables|Default|GetLine%20Trace%20Distance))) "TraceTypeQuery1" false (Utilities|Array|MakeArray (Components|GetOwner Ak%20Component)) "None"))
  (if _returnvalue_2
    (return (Variables|/Script/PhysicsCore.PhysicalMaterial|GetSurfaceType (.PhysMat (Collision|BreakHitResult _outhit))) true)))

(fn GetEventtoPost
  (switch Utilities|FlowControl|Switch|SwitchonEFootstepType (Variables|Default|GetFootstep%20Type)
    (:NewEnumerator0
      (LocalVariables|SetAk%20Event "/Game/Sound/Wwise/Events/Testing/Beeps/Play_test_beep_short.Play_test_beep_short"))
    (:NewEnumerator1
      (LocalVariables|SetAk%20Event 0))
    (:NewEnumerator2
      (LocalVariables|SetAk%20Event 0))
    (:NewEnumerator3
      (LocalVariables|SetAk%20Event 0)))
  (return (LocalVariables|GetAk%20Event)))

(fn PostEvent
  (params (Ak%20Component :type Ak%20Component%20Object%20Reference%20%28by%20ref%29))
  (bind _akevent (CallFunction|GetEventtoPost))
  (Utilities|IsValid _akevent
    (:Is%20Valid
      (Class|AkGameObject|PostAkEvent Ak%20Component _akevent))))

(fn GetNotifyName
  (return (Utilities|String|Append "SND_Fst_" (Utilities|String|EnumtoString (Variables|Default|GetFootstep%20Type)))))